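; BP_Spawner1 is a spawner actor that populates the area around itself with BP_SimpleMolecule actors.
; On BeginPlay, a short fixed loop spawns the molecules, each at a freshly randomized location.
; GetSpawnLocation offsets the spawner's position by an independent random amount on each axis within a given spread, so spawns scatter inside a cube centered on the actor.
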(event EventBeginPlay
  (for _index (range 0 2)
    (Game|SpawnActorfromClass "/Game/BP_SimpleMolecule.BP_SimpleMolecule_C" (Math|Transform|MakeTransform (CallFunction|GetSpawnLocation 7e+01) "0, 0, 0" "1,1,1") "Undefined" 0 0)))

(fn ConstructionScript)

(fn GetSpawnLocation
  (params (Spread :type Float%20%28single-precision%29))
  (bind _returnvalue (- 0.0 Spread))
  (bind _returnvalue_2 (Transformation|GetActorLocation))
  (return (Math|Vector|MakeVector (+ (.x _returnvalue_2) (Math|Random|RandomFloatinRange _returnvalue Spread)) (+ (.y _returnvalue_2) (Math|Random|RandomFloatinRange _returnvalue Spread)) (+ (.z _returnvalue_2) (Math|Random|RandomFloatinRange _returnvalue Spread)))))