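; BP_Atom is a physics-driven atom actor that repels or attracts other atoms depending on their distance.
; Each tick it finds atoms overlapping its Sphere, excludes itself, and applies a force to PhysicsMesh along the line between them.
; CalculateForceFromDistance uses a Lennard-Jones-style pair of opposing inverse power terms, clamped to limit extreme forces.
; Each computed force is also printed for debugging.
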(event EventBeginPlay)

(event Collision|EventActorBeginOverlap
  (params (OtherActor :type Actor%20Object%20Reference)))

(event EventTick
  (params (DeltaSeconds :type Float%20%28single-precision%29))
  (for _array_element (Collision|GetOverlappingActors (Variables|Default|GetSphere) "BP_Atom_C" :!class /Script/Engine.PrimitiveComponent)
    (bind _objectout (Utilities|IsAtomNotSelf _array_element))
    (Development|PrintString (Utilities|String|ToString(Float) (CallFunction|CalculateForcefromDistance (Math|Vector|VectorLength (- (Transformation|GetWorldLocation (Variables|Default|GetPhysicsMesh)) (Transformation|GetWorldLocation (Variables|/Script/MoleculePrototype.Atom|GetPhysicsMesh _objectout)))))))
    (Physics|AddForce (Variables|Default|GetPhysicsMesh) (* (Math|Vector|Normalize (- (Transformation|GetWorldLocation (Variables|Default|GetPhysicsMesh)) (Transformation|GetWorldLocation (Variables|/Script/MoleculePrototype.Atom|GetPhysicsMesh _objectout)))) (CallFunction|CalculateForcefromDistance (Math|Vector|VectorLength (- (Transformation|GetWorldLocation (Variables|Default|GetPhysicsMesh)) (Transformation|GetWorldLocation (Variables|/Script/MoleculePrototype.Atom|GetPhysicsMesh _objectout)))))) "None" false)))

(fn ConstructionScript)

(fn CalculateForcefromDistance
  (params (Distance :type Float%20%28single-precision%29))
  (bind _returnvalue (Math|Float|MakeLiteralFloat 1e+04))
  (bind _returnvalue_2 (/ Distance 1e+01))
  (return (Math|Float|Clamp(Float) (* (+ (/ (Math|Float|MakeLiteralFloat 435211337728.0) (Math|Float|Power _returnvalue_2 7.5)) (/ (Math|Float|MakeLiteralFloat -137567076352.0) (Math|Float|Power _returnvalue_2 7.0))) 4.6) (* -1 _returnvalue) _returnvalue)))