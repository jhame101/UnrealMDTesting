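; BP_SimpleMolecule is a molecule made of two atom child actor components joined by a single bond.
; On BeginPlay it calls CreateBond on Atom1 and Atom2 with BP_SingleBond, then zeroes LaunchStrength.
; A deprecated local bond function remains, which casts both child actors to Atom, spawns the bond and attaches it, printing a warning if a cast fails.
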(event EventBeginPlay
  (Class|BondBase|CreateBond (Variables|Default|GetAtom1) (Variables|Default|GetAtom2) "/Game/BP_SingleBond.BP_SingleBond_C")
  (Variables|Default|SetLaunchStrength 0.0))

(fn ConstructionScript)

(fn DEPRECATEDCreateBond
  (params (ChildAtomComponent1 :type Child%20Actor%20Component%20Object%20Reference) (ChildAtomComponent2 :type Child%20Actor%20Component%20Object%20Reference) (BondClass :type Bond%20Base%20Class%20Reference))
  (bind _asatom (Utilities|Casting|CastToAtom (Variables|/Script/Engine.ChildActorComponent|GetChildActor ChildAtomComponent2))
    (:then
      (bind _asatom_2 (Utilities|Casting|CastToAtom (Variables|/Script/Engine.ChildActorComponent|GetChildActor ChildAtomComponent1))
        (:then
          (bind _returnvalue (Game|SpawnActorfromClass BondClass (Math|Transform|MakeTransform "0, 0, 0" "0, 0, 0" "1,1,1") "Undefined" 0 0))
          (Class|BondBase|AttachtoAtoms _returnvalue _asatom_2 _asatom)
          (return _asatom_2 _asatom _returnvalue))
        (:CastFailed
          _)))
    (:CastFailed
      _))
  (Development|PrintString (Utilities|String|MakeLiteralString "Warning: one or both child actors are not an atom") true true "(R=1.000000,G=0.000000,B=0.000000,A=1.000000)" 1e+01)
  (return 0 0 0))