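; BP_SpawnerSeperate is a spawner actor that creates two bonded BP_Atom actors at random positions around itself on BeginPlay.
; GetSpawnLocation randomizes each axis within a spread, and is re-evaluated for each atom, so the small opposing Z offsets do not keep the pair together.
; A spawned BP_SingleBond links the two half-scale atoms through AttachToAtoms.
; A loop for repeating the spawn fifty times is disconnected, so only one pair spawns.
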(event EventBeginPlay
  (bind _spawnlocation (CallFunction|GetSpawnLocation 3e+02))
  (bind _returnvalue (Game|SpawnActorfromClass "/Game/Atoms/BP_Atom.BP_Atom_C" (Math|Transform|MakeTransform (Math|Vector|MakeVector (.x _spawnlocation) (.y _spawnlocation) (+ (.z _spawnlocation) 0.5)) "0, 0, 0" "0.500000,0.500000,0.500000") "AdjustIfPossibleButAlwaysSpawn" 0 0))
  (bind _returnvalue_2 (Game|SpawnActorfromClass "/Game/Atoms/BP_Atom.BP_Atom_C" (Math|Transform|MakeTransform (Math|Vector|MakeVector (.x _spawnlocation) (.y _spawnlocation) (- (.z _spawnlocation) 0.5)) "0, 0, 0" "0.500000,0.500000,0.500000") "AdjustIfPossibleButAlwaysSpawn" 0 0))
  (bind _returnvalue_3 (Game|SpawnActorfromClass "/Game/BP_SingleBond.BP_SingleBond_C" (Math|Transform|MakeTransform "0, 0, 0" "0, 0, 0" "1,1,1") "AlwaysSpawn" 0 0))
  (Class|BondBase|AttachtoAtoms _returnvalue_3 _returnvalue_2 _returnvalue))

(fn ConstructionScript)

(fn GetSpawnLocation
  (params (Spread :type Float%20%28single-precision%29))
  (bind _returnvalue (- 0.0 Spread))
  (bind _returnvalue_2 (Transformation|GetActorLocation))
  (return (Math|Vector|MakeVector (+ (.x _returnvalue_2) (Math|Random|RandomFloatinRange _returnvalue Spread)) (+ (.y _returnvalue_2) (Math|Random|RandomFloatinRange _returnvalue Spread)) (+ (.z _returnvalue_2) (Math|Random|RandomFloatinRange _returnvalue Spread)))))